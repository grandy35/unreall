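; BP_ball is a ball actor that moves in a straight line and bounces off surfaces it hits.
; Each Tick it sweeps its Sphere component along Direction, scaled by Speed and delta time.
; It then mirrors Direction around the sweep's hit normal, behind a branch whose condition is a constant true rather than a blocking-hit check.
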(event `self.ReceiveTick`
  (params (DeltaSeconds :type "Float (single-precision)"))
  (bind _sweephitresult (`SceneComponent.K2_AddWorldOffset` (`self.Sphere`) (* (* (`self.Direction`) (`self.Speed`)) DeltaSeconds) true false))
  (if true
    (set `self.Direction` (`KismetMathLibrary.GetReflectionVector` (`self.Direction`) (`.Normal` (`GameplayStatics.BreakHitResult` _sweephitresult))))))

(fn `UserConstructionScript`)